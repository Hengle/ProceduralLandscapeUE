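; Landscape brush Blueprint that stamps a heightmap texture onto terrain, with adjustable UV offset, rotation, fade and radius of influence.
; DoesBrushNeedRedraw compares settings, yaw and up vector against cached past values, using tolerances for offset and tilt.
; Changes are pushed to the brush and layer-brush dynamic materials, and RedrawNeed is flagged to redraw the landscape.
; ResetBrush restores the cached values to fixed defaults.
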(event EventBeginPlay)

(event EventTick
  (params (DeltaSeconds :type Float%20%28single-precision%29)))

(event EventDoesBrushNeedRedraw
  (bind _returnvalue (Transformation|GetActorRotation))
  (bind _returnvalue_2 (Transformation|GetActorUpVector))
  (bind _radiusofinfluencemeters (Variables|Default|GetRadiusOfInfluenceMeters))
  (bind _fadeamount (Variables|Default|GetFadeAmount))
  (bind _heightmap (Variables|Default|GetHeightMap))
  (bind _heightmap_2 (Variables|Default|GetHeightMap))
  (bind _heightmapdatamap (Variables|Default|GetHeightMapDataMap))
  (bind _heightmapdatamap_2 (Variables|Default|GetHeightMapDataMap))
  (bind _fadeoutstartunit (Variables|Default|GetFadeOutStartUnit))
  (bind _yaw (Math|Rotator|BreakRotator _returnvalue))
  (Utilities|FlowControl|Sequence
    (:then_0
      (if (> (Math|Vector|VectorLength (- (Variables|Default|GetUVOffset) (Variables|Past|GetUVOffset_past))) 0.01)
        (bind _output_get (Variables|Past|SetUVOffset_past (Variables|Default|GetUVOffset)))
        (Utilities|FlowControl|Sequence
          (:then_0
            (bind _returnvalue_3 (Class|ShaderWorldBrush|GetBrushDynamicMaterial))
            (Utilities|IsValid _returnvalue_3
              (:Is%20Valid
                (Rendering|Material|SetVectorParameterValue _returnvalue_3 "UVOffset" (Math|Conversions|ToLinearColor(Vector) _output_get) :!class /Script/Engine.MaterialInstanceDynamic)
                ;[0.9477 1 0] We are asking for landscape redraw
                (Variables|Default|SetRedrawNeed true))))
          (:then_1
            (bind _returnvalue_4 (Class|ShaderWorldBrush|GetLayerBrushDynamicMaterial))
            (Utilities|IsValid _returnvalue_4
              (:Is%20Valid
                (Rendering|Material|SetVectorParameterValue _returnvalue_4 "UVOffset" (Math|Conversions|ToLinearColor(Vector) _output_get) :!class /Script/Engine.MaterialInstanceDynamic)))))))
    (:then_1
      (if (!= _yaw (Variables|past|Getyaw_past))
        (Variables|past|Setyaw_past _yaw)
        (Utilities|FlowControl|Sequence
          (:then_0
            (bind _returnvalue_5 (Class|ShaderWorldBrush|GetBrushDynamicMaterial))
            (Utilities|IsValid _returnvalue_5
              (:Is%20Valid
                (Rendering|Material|SetScalarParameterValue _returnvalue_5 "BrushYaw" _yaw :!class /Script/Engine.MaterialInstanceDynamic)
                ;[0.9477 1 0] We are asking for landscape redraw
                (Variables|Default|SetRedrawNeed true))))
          (:then_1
            (bind _returnvalue_6 (Class|ShaderWorldBrush|GetLayerBrushDynamicMaterial))
            (Utilities|IsValid _returnvalue_6
              (:Is%20Valid
                (Rendering|Material|SetScalarParameterValue _returnvalue_6 "BrushYaw" _yaw :!class /Script/Engine.MaterialInstanceDynamic)))))))
    (:then_2
      (if (!= (Variables|Default|GetFadeAmount) (Variables|Past|GetFadeAmount_past))
        (Variables|Past|SetFadeAmount_past (Variables|Default|GetFadeAmount))
        (Utilities|FlowControl|Sequence
          (:then_0
            (bind _returnvalue_7 (Class|ShaderWorldBrush|GetBrushDynamicMaterial))
            (Utilities|IsValid _returnvalue_7
              (:Is%20Valid
                (Rendering|Material|SetScalarParameterValue _returnvalue_7 "FadeAmount" _fadeamount :!class /Script/Engine.MaterialInstanceDynamic)
                ;[0.9477 1 0] We are asking for landscape redraw
                (Variables|Default|SetRedrawNeed true))))
          (:then_1
            (bind _returnvalue_8 (Class|ShaderWorldBrush|GetLayerBrushDynamicMaterial))
            (Utilities|IsValid _returnvalue_8
              (:Is%20Valid
                (Rendering|Material|SetScalarParameterValue _returnvalue_8 "FadeAmount" _fadeamount :!class /Script/Engine.MaterialInstanceDynamic)))))))
    (:then_3
      (if (!= (Variables|Default|GetFadeOutStartUnit) (Variables|Past|GetFadeOutStartUnit_past))
        (Variables|Past|SetFadeOutStartUnit_past (Variables|Default|GetFadeOutStartUnit))
        (Utilities|FlowControl|Sequence
          (:then_0
            (bind _returnvalue_9 (Class|ShaderWorldBrush|GetBrushDynamicMaterial))
            (Utilities|IsValid _returnvalue_9
              (:Is%20Valid
                (Rendering|Material|SetScalarParameterValue _returnvalue_9 "FadeOutStartUnit" _fadeoutstartunit :!class /Script/Engine.MaterialInstanceDynamic)
                ;[0.9477 1 0] We are asking for landscape redraw
                (Variables|Default|SetRedrawNeed true))))
          (:then_1
            (bind _returnvalue_10 (Class|ShaderWorldBrush|GetLayerBrushDynamicMaterial))
            (Utilities|IsValid _returnvalue_10
              (:Is%20Valid
                (Rendering|Material|SetScalarParameterValue _returnvalue_10 "FadeOutStartUnit" _fadeoutstartunit :!class /Script/Engine.MaterialInstanceDynamic)))))))
    (:then_4
      (if (< (Math|Vector|DotProduct _returnvalue_2 (Variables|Past|GetBrushUpVector_past)) 0.99)
        (bind _output_get_2 (Variables|Past|SetBrushUpVector_past _returnvalue_2))
        (Utilities|FlowControl|Sequence
          (:then_0
            (bind _returnvalue_11 (Class|ShaderWorldBrush|GetBrushDynamicMaterial))
            (Utilities|IsValid _returnvalue_11
              (:Is%20Valid
                (Rendering|Material|SetVectorParameterValue _returnvalue_11 "BrushUpVector" (Math|Conversions|ToLinearColor(Vector) _output_get_2) :!class /Script/Engine.MaterialInstanceDynamic)
                ;[0.9477 1 0] We are asking for landscape redraw
                (Variables|Default|SetRedrawNeed true))))
          (:then_1
            (bind _returnvalue_12 (Class|ShaderWorldBrush|GetLayerBrushDynamicMaterial))
            (Utilities|IsValid _returnvalue_12
              (:Is%20Valid
                (Rendering|Material|SetVectorParameterValue _returnvalue_12 "BrushUpVector" (Math|Conversions|ToLinearColor(Vector) _output_get_2) :!class /Script/Engine.MaterialInstanceDynamic)))))))
    (:then_5
      (Utilities|IsValid _heightmap
        (:Is%20Valid
          (if (!= _heightmap (Variables|Past|GetHeightMap_past))
            (Variables|Past|SetHeightMap_past (Variables|Default|GetHeightMap))
            (Utilities|FlowControl|Sequence
              (:then_0
                (bind _returnvalue_13 (Class|ShaderWorldBrush|GetBrushDynamicMaterial))
                (Utilities|IsValid _returnvalue_13
                  (:Is%20Valid
                    (Rendering|Material|SetTextureParameterValue _returnvalue_13 "HeightMapBrush" _heightmap_2))))
              (:then_1
                (bind _returnvalue_14 (Class|ShaderWorldBrush|GetLayerBrushDynamicMaterial))
                (Utilities|IsValid _returnvalue_14
                  (:Is%20Valid
                    (Rendering|Material|SetTextureParameterValue _returnvalue_14 "HeightMapBrush" _heightmap_2)))))
            ;[0.9477 1 0] We are asking for landscape redraw
            (Variables|Default|SetRedrawNeed true)))))
    (:then_6
      (Utilities|IsValid _heightmapdatamap
        (:Is%20Valid
          (if (!= _heightmapdatamap (Variables|Past|GetHeightMapDataMap_past))
            (Variables|Past|SetHeightMapDataMap_past (Variables|Default|GetHeightMapDataMap))
            (Utilities|FlowControl|Sequence
              (:then_0
                (bind _returnvalue_15 (Class|ShaderWorldBrush|GetBrushDynamicMaterial))
                (Utilities|IsValid _returnvalue_15
                  (:Is%20Valid
                    (Rendering|Material|SetTextureParameterValue _returnvalue_15 "HeightMapData" _heightmapdatamap_2)
                    ;[0.9477 1 0] We are asking for landscape redraw
                    (Variables|Default|SetRedrawNeed true))))
              (:then_1
                (bind _returnvalue_16 (Class|ShaderWorldBrush|GetLayerBrushDynamicMaterial))
                (Utilities|IsValid _returnvalue_16
                  (:Is%20Valid
                    (Rendering|Material|SetTextureParameterValue _returnvalue_16 "HeightMapData" _heightmapdatamap_2)))))))))
    (:then_7
      (if (!= (Variables|Default|GetRadiusOfInfluenceMeters) (Variables|Past|GetRadiusOfInfluence_past))
        (Variables|Past|SetRadiusOfInfluence_past (Variables|Default|GetRadiusOfInfluenceMeters))
        (Utilities|FlowControl|Sequence
          (:then_0
            (bind _returnvalue_17 (Class|ShaderWorldBrush|GetBrushDynamicMaterial))
            (Utilities|IsValid _returnvalue_17
              (:Is%20Valid
                (Rendering|Material|SetScalarParameterValue _returnvalue_17 "InfluenceRadius" _radiusofinfluencemeters :!class /Script/Engine.MaterialInstanceDynamic)
                ;[0.9477 1 0] We are asking for landscape redraw
                (Variables|Default|SetRedrawNeed true))))
          (:then_1
            (bind _returnvalue_18 (Class|ShaderWorldBrush|GetLayerBrushDynamicMaterial))
            (Utilities|IsValid _returnvalue_18
              (:Is%20Valid
                (Rendering|Material|SetScalarParameterValue _returnvalue_18 "InfluenceRadius" _radiusofinfluencemeters :!class /Script/Engine.MaterialInstanceDynamic)))))))))

(event EventResetBrush
  (Utilities|FlowControl|Sequence
    (:then_0
      (Variables|past|Setyaw_past 0.0))
    (:then_1
      (Variables|Past|SetUVOffset_past "0, 0, 0"))
    (:then_2
      (Variables|Past|SetFadeAmount_past 2e+01))
    (:then_3
      (Variables|Past|SetFadeOutStartUnit_past 0.8))
    (:then_4
      (Variables|Past|SetBrushUpVector_past "0, 0,1.000000"))
    (:then_5
      (Variables|Past|SetRadiusOfInfluence_past 1e+03))
    (:then_6
      (Variables|Past|SetHeightMapDataMap_past "/Engine/EngineResources/DefaultTexture.DefaultTexture"))
    (:then_7
      (Variables|Past|SetHeightMap_past "/Engine/EngineResources/DefaultTexture.DefaultTexture"))))

(fn ConstructionScript)