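; BP_BrushDemo is a demo landscape brush that exposes invert and influence radius controls.
; DoesBrushNeedRedraw checks both settings, writes changes to the brush's dynamic material parameters and flags the landscape for redraw.
; Paired DoOnce nodes limit updates to Invert toggles, and a cached past value detects radius changes.
; An author note recommends C++ for frequently changing parameters, as Blueprint calls are expensive.
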(event EventBeginPlay)

(event EventTick
  (params (DeltaSeconds :type Float%20%28single-precision%29)))

(event EventDoesBrushNeedRedraw
  ;[1 0.233 0.1166] For parameters changing regularly it's recommended to use c++ as blueprint calls are performance expensive
  (Utilities|FlowControl|Sequence
    (:then_0
      (if (Variables|Default|GetInvert)
        (Utilities|FlowControl|DoOnce false :!label _label
          (:Completed
            (Utilities|FlowControl|Sequence
              (:then_0
                _)
              (:then_1
                (goto _label_2 Reset)))))
        (else
          (Utilities|FlowControl|DoOnce false :!label _label_2
            (:Completed
              (Utilities|FlowControl|Sequence
                (:then_0
                  _)
                (:then_1
                  (goto _label Reset)))))))
      (bind _returnvalue (Class|ShaderWorldBrush|GetBrushDynamicMaterial))
      (Utilities|IsValid _returnvalue
        (:Is%20Valid
          (Rendering|Material|SetScalarParameterValue _returnvalue "Invert" (Math|Float|SelectFloat -1.0 1.0 (Variables|Default|GetInvert)) :!class /Script/Engine.MaterialInstanceDynamic)
          ;[0.9477 1 0] We are asking for landscape redraw
          (Variables|Default|SetRedrawNeed true))))
    (:then_1
      (if (!= (Variables|Default|GetInfluenceRadius) (Variables|past|GetInfluenceRadius_past))
        (Variables|past|SetInfluenceRadius_past (Variables|Default|GetInfluenceRadius))
        (bind _returnvalue_2 (Class|ShaderWorldBrush|GetBrushDynamicMaterial))
        (Utilities|IsValid _returnvalue_2
          (:Is%20Valid
            (Rendering|Material|SetScalarParameterValue _returnvalue_2 "InfluenceRadius" (Variables|Default|GetInfluenceRadius) :!class /Script/Engine.MaterialInstanceDynamic)
            ;[0.9477 1 0] We are asking for landscape redraw
            (Variables|Default|SetRedrawNeed true)))))))

(event EventResetBrush
  ;[1 1 1] If you have some cleaning to do
)

(fn ConstructionScript)